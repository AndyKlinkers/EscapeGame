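; Player controller for an escape game that manages the inventory screen.
; The OpenInventory input toggles a WB_Inventory widget in the viewport, creating it on first use and reusing the cached instance afterwards.
; A ReloadInventory event tells that cached widget to reload its items, and does nothing if the widget has not been created.
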(event EventReloadInventory
  (bind _inventory_widget (Variables|Default|GetInventory%20widget))
  (Utilities|IsValid _inventory_widget
    (:Is%20Valid
      (bind _aswb_inventory (Utilities|Casting|CastToWB_Inventory _inventory_widget))
      (Default|LoadInventoryItems _aswb_inventory))))

(event Input|ActionEvents|InputActionOpenInventory
  (params (Key :type Key%20Structure))
  (:Pressed
    (if (Utilities|IsValid (Variables|Default|GetInventory%20widget))
      (if (Widget|IsVisible (Variables|Default|GetInventory%20widget))
        (Widget|RemovefromParent (Variables|Default|GetInventory%20widget))
        (else
          (Utilities|IsValid (Variables|Default|GetInventory%20widget)
            (:Is%20Valid
              (UserInterface|Viewport|AddtoViewport (Variables|Default|GetInventory%20widget) 0 :!label _label)))))
      (else
        (bind _returnvalue (UserInterface|CreateWidget "/Game/UI/WB_Inventory.WB_Inventory_C"))
        (Variables|Default|SetInventory%20widget _returnvalue)
        (goto _label)))))

(fn ConstructionScript)